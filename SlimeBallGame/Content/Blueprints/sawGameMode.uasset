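; sawGameMode is a game mode that tracks score and lives and shows them on a HUD.
; On BeginPlay it creates the ScoreandLives widget, adds it to the viewport and calls ResetTubes, which restores lives to the maximum and zeroes points.
; UpdateScore adds a delta to the current points, clamps the total at zero and pushes it to the HUD.
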(event Custom|UpdateScore
  (params (Points :type Integer))
  ;[1 1 1] Update score
  (if (<= (+ Points (Variables|Default|GetCurrentPoints)) 0)
    (Variables|Default|SetCurrentPoints 0)
    (else
      (Variables|Default|SetCurrentPoints (+ Points (Variables|Default|GetCurrentPoints)))))
  (Variables|/Game/Blueprints/UI/ScoreandLives.ScoreandLives_C|SetPoints (Variables|Default|GetHUD) (Variables|Default|GetCurrentPoints)))

(event Custom|ResetTubes
  (bind _maxlives (Variables|Default|GetMaxLives))
  (bind _hud (Variables|Default|GetHUD))
  ;[1 1 1] Reset Game
  (Variables|Default|SetLives _maxlives)
  (Variables|/Game/Blueprints/UI/ScoreandLives.ScoreandLives_C|SetLives _hud _maxlives)
  (Variables|/Game/Blueprints/UI/ScoreandLives.ScoreandLives_C|SetPoints _hud 0)
  (Variables|Default|SetCurrentPoints 0))

(event EventBeginPlay
  ;[1 1 1] Add HUD
  (bind _returnvalue (UserInterface|CreateWidget "/Game/Blueprints/UI/ScoreandLives.ScoreandLives_C"))
  (bind _output_get (Variables|Default|SetHUD _returnvalue))
  (UserInterface|Viewport|AddtoViewport _output_get 0)
  (CallFunction|ResetTubes))

(fn ConstructionScript)

(fn Reset)