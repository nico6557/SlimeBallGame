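; Goal actor that destroys slimes overlapping its Killbox and awards Points to the score.
; Fire, lightning and radioactive slimes score on overlap, while hero slimes use a SecondHero toggle to count only every second overlap, as a duplicate check.
; AddPoints finds the active game mode through a cast chain and calls its UpdateScore.
; Only mainGameMode also has its objective goal decremented.
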(event OnComponentBeginOverlap(killbox)
  (params (OverlappedComponent :type Primitive%20Component%20Object%20Reference) (OtherActor :type Actor%20Object%20Reference) (OtherComp :type Primitive%20Component%20Object%20Reference) (OtherBodyIndex :type Integer) (bFromSweep :type Boolean) (SweepResult :type Hit%20Result%20Structure%20%28by%20ref%29))
  (CallFunction|CheckforSlime OtherActor))

(event Custom|Add%20Points
  ;[1 1 1] Adds points to the score
  (bind _asmain_game_mode (Utilities|Casting|CastTomainGameMode (Game|GetGameMode))
    (:then
      (Default|UpdateScore _asmain_game_mode (Variables|Default|GetPoints))
      (Default|UpdateObjectiveGoal _asmain_game_mode -1))
    (:CastFailed
      (bind _astubes_game_mode (Utilities|Casting|CastTotubesGameMode (Game|GetGameMode))
        (:then
          (Default|UpdateScore _astubes_game_mode (Variables|Default|GetPoints)))
        (:CastFailed
          (bind _asmonster_game_mode (Utilities|Casting|CastTomonsterGameMode (Game|GetGameMode))
            (:then
              (Default|UpdateScore _asmonster_game_mode (Variables|Default|GetPoints)))
            (:CastFailed
              (bind _asgoblin_camp_game_mode (Utilities|Casting|CastTogoblinCampGameMode (Game|GetGameMode))
                (:then
                  (Default|UpdateScore _asgoblin_camp_game_mode (Variables|Default|GetPoints)))
                (:CastFailed
                  (bind _asboss_game_mode (Utilities|Casting|CastTobossGameMode (Game|GetGameMode))
                    (:then
                      (Default|UpdateScore _asboss_game_mode (Variables|Default|GetPoints)))
                    (:CastFailed
                      (bind _assaw_game_mode (Utilities|Casting|CastTosawGameMode (Game|GetGameMode)))
                      (Default|UpdateScore _assaw_game_mode (Variables|Default|GetPoints)))))))))))))

(event Custom|Check%20for%20Slime
  (params (Slime :type Actor%20Object%20Reference))
  ;[1 1 1] Check for duplicate
  (bind _ashero_slime_bp (Utilities|Casting|CastToheroSlimeBP Slime)
    (:then
      (if (Variables|Default|GetSecondHero)
        (Actor|DestroyActor _ashero_slime_bp)
        (Variables|Default|SetSecondHero false)
        (CallFunction|AddPoints)
        (else
          (Variables|Default|SetSecondHero true))))
    (:CastFailed
      (bind _asfire_slime_bp (Utilities|Casting|CastTofireSlimeBP Slime)
        (:then
          (Actor|DestroyActor _asfire_slime_bp)
          (CallFunction|AddPoints))
        (:CastFailed
          (bind _aslightning_slime_bp (Utilities|Casting|CastTolightningSlimeBP Slime)
            (:then
              (Actor|DestroyActor _aslightning_slime_bp)
              (CallFunction|AddPoints))
            (:CastFailed
              (bind _asradioactive_slime_bp (Utilities|Casting|CastToradioactiveSlimeBP Slime))
              (Actor|DestroyActor _asradioactive_slime_bp)
              (CallFunction|AddPoints))))))))

(event EventBeginPlay)

(event Collision|EventActorBeginOverlap
  (params (OtherActor :type Actor%20Object%20Reference)))

(event EventTick
  (params (DeltaSeconds :type Float%20%28single-precision%29)))

(fn ConstructionScript)