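; Game mode for a monster level with a break-teeth objective, tracking score, lives and objective progress.
; On BeginPlay it creates the score/lives and objective HUD widgets, then resets their displayed values.
; Update events add deltas to the stored values, flooring score at zero and capping lives and objective, then push them to the widgets.
; When lives or the objective count reaches zero, it shows the level selector widget.
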(event Custom|UpdateScore
  (params (Points :type Integer))
  ;[1 1 1] Update score
  (if (<= (+ Points (Variables|Default|GetCurrentPoints)) 0)
    (Variables|Default|SetCurrentPoints 0)
    (else
      (Variables|Default|SetCurrentPoints (+ Points (Variables|Default|GetCurrentPoints)))))
  (Variables|/Game/Blueprints/UI/ScoreandLives.ScoreandLives_C|SetPoints (Variables|Default|GetHUD) (Variables|Default|GetCurrentPoints)))

(event Custom|UpdateLives
  (params (LivesLeft :type Integer))
  ;[1 1 1] Update Objective Save
  (if (>= (+ LivesLeft (Variables|Default|GetLives)) 8)
    (Variables|Default|SetLives 8)
    (else
      (Variables|Default|SetLives (+ LivesLeft (Variables|Default|GetLives)))))
  (bind _output_get (Variables|/Game/Blueprints/UI/ScoreandLives.ScoreandLives_C|SetLives (Variables|Default|GetHUD) (Variables|Default|GetLives)))
  (if (<= _output_get 0)
    (bind _returnvalue (UserInterface|CreateWidget "/Game/Blueprints/UI/levelSelector.levelSelector_C"))
    (UserInterface|Viewport|AddtoViewport _returnvalue 0)))

(event Custom|ResetMonster
  (bind _hud (Variables|Default|GetHUD))
  ;[1 1 1] Reset Game
  (Variables|Default|SetMaxLives (Variables|Default|GetMaxLives))
  (Variables|/Game/Blueprints/UI/ScoreandLives.ScoreandLives_C|SetLives _hud (Variables|Default|GetMaxLives))
  (Variables|/Game/Blueprints/UI/ScoreandLives.ScoreandLives_C|SetPoints _hud 0)
  (Variables|/Game/Blueprints/UI/ObjectiveBreakTeeth.ObjectiveBreakTeeth_C|SetObjective (Variables|Default|GetOBJHUD) 10)
  (Variables|Default|SetCurrentPoints 0))

(event Custom|UpdateObjectiveBreak
  (params (Objective :type Integer))
  ;[1 1 1] Update Objective Save
  (if (>= (+ Objective (Variables|Default|GetgoalObjective)) 10)
    (Variables|Default|SetgoalObjective 10)
    (else
      (Variables|Default|SetgoalObjective (+ Objective (Variables|Default|GetgoalObjective)))))
  (bind _output_get (Variables|/Game/Blueprints/UI/ObjectiveBreakTeeth.ObjectiveBreakTeeth_C|SetObjective (Variables|Default|GetOBJHUD) (Variables|Default|GetgoalObjective)))
  (if (<= _output_get 0)
    (bind _returnvalue (UserInterface|CreateWidget "/Game/Blueprints/UI/levelSelector.levelSelector_C"))
    (UserInterface|Viewport|AddtoViewport _returnvalue 0)))

(event EventBeginPlay
  ;[1 1 1] Add HUD
  (bind _returnvalue (UserInterface|CreateWidget "/Game/Blueprints/UI/ScoreandLives.ScoreandLives_C"))
  (bind _output_get (Variables|Default|SetHUD _returnvalue))
  (UserInterface|Viewport|AddtoViewport _output_get 0)
  (bind _returnvalue_2 (UserInterface|CreateWidget "/Game/Blueprints/UI/ObjectiveBreakTeeth.ObjectiveBreakTeeth_C"))
  (bind _output_get_2 (Variables|Default|SetOBJHUD _returnvalue_2))
  (UserInterface|Viewport|AddtoViewport _output_get_2 0)
  (CallFunction|ResetMonster))

(fn ConstructionScript)

(fn Reset)