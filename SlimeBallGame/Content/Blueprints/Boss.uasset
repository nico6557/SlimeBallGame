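; Boss actor that loses health when hit by slimes, awarding points and breaking with a bloop sound at zero health.
; Sphere overlaps from hero, radioactive or lightning slimes each decrement BossHealth; fire slime branches are disconnected.
; AddPoints, called per hit and again on death, tries six game mode casts to update score.
; In bossGameMode, each call also decrements the boss objective.
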(event OnComponentBeginOverlap(Sphere)
  (params (OverlappedComponent :type Primitive%20Component%20Object%20Reference) (OtherActor :type Actor%20Object%20Reference) (OtherComp :type Primitive%20Component%20Object%20Reference) (OtherBodyIndex :type Integer) (bFromSweep :type Boolean) (SweepResult :type Hit%20Result%20Structure%20%28by%20ref%29))
  ;[1 1 1] on second hit the sphere breaks playiong a noise
  (Utilities|IsValid OtherActor
    (:Is%20Valid
      ;[1 1 1] on second hit the sphere breaks playiong a noise
      (Utilities|Casting|CastToheroSlimeBP OtherActor
        (:then
          (Math|Integer|DecrementInt (Variables|Default|GetBossHealth)
            (:%20%20
              (CallFunction|AddPoints)
              (if (== (Variables|Default|GetBossHealth) 0)
                (Utilities|FlowControl|Delay 0.1)
                (Actor|DestroyActor self)
                (CallFunction|AddPoints)
                (Audio|PlaySoundatLocation "/Game/Sounds/bloopCue.bloopCue" "0, 0, 0" "0, 0, 0" 1.0 1.0 0.0 0 0 0)))))
        (:CastFailed
          ;[1 1 1] on second hit the sphere breaks playiong a noise
          (Utilities|Casting|CastToradioactiveSlimeBP OtherActor
            (:then
              (Math|Integer|DecrementInt (Variables|Default|GetBossHealth)
                (:%20%20
                  (CallFunction|AddPoints)
                  (if (== (Variables|Default|GetBossHealth) 0)
                    (Utilities|FlowControl|Delay 0.1)
                    (Actor|DestroyActor self)
                    (CallFunction|AddPoints)
                    (Audio|PlaySoundatLocation "/Game/Sounds/bloopCue.bloopCue" "0, 0, 0" "0, 0, 0" 1.0 1.0 0.0 0 0 0)))))
            (:CastFailed
              ;[1 1 1] on second hit the sphere breaks playiong a noise
              (Utilities|Casting|CastTolightningSlimeBP OtherActor)
              (Math|Integer|DecrementInt (Variables|Default|GetBossHealth)
                (:%20%20
                  (CallFunction|AddPoints)
                  (if (== (Variables|Default|GetBossHealth) 0)
                    (Utilities|FlowControl|Delay 0.1)
                    (Actor|DestroyActor self)
                    (CallFunction|AddPoints)
                    (Audio|PlaySoundatLocation "/Game/Sounds/bloopCue.bloopCue" "0, 0, 0" "0, 0, 0" 1.0 1.0 0.0 0 0 0)))))))))))

(event Custom|Add%20Points
  ;[1 1 1] Adds points to the score
  (bind _asmain_game_mode (Utilities|Casting|CastTomainGameMode (Game|GetGameMode))
    (:then
      (Default|UpdateScore _asmain_game_mode (Variables|Default|GetPoints)))
    (:CastFailed
      (bind _astubes_game_mode (Utilities|Casting|CastTotubesGameMode (Game|GetGameMode))
        (:then
          (Default|UpdateScore _astubes_game_mode (Variables|Default|GetPoints)))
        (:CastFailed
          (bind _asmonster_game_mode (Utilities|Casting|CastTomonsterGameMode (Game|GetGameMode))
            (:then
              (Default|UpdateScore _asmonster_game_mode (Variables|Default|GetPoints)))
            (:CastFailed
              (bind _asgoblin_camp_game_mode (Utilities|Casting|CastTogoblinCampGameMode (Game|GetGameMode))
                (:then
                  (Default|UpdateScore _asgoblin_camp_game_mode (Variables|Default|GetPoints)))
                (:CastFailed
                  (bind _asboss_game_mode (Utilities|Casting|CastTobossGameMode (Game|GetGameMode))
                    (:then
                      (Default|UpdateScore _asboss_game_mode (Variables|Default|GetPoints))
                      (Default|UpdateObjectiveBoss _asboss_game_mode -1))
                    (:CastFailed
                      (bind _assaw_game_mode (Utilities|Casting|CastTosawGameMode (Game|GetGameMode)))
                      (Default|UpdateScore _assaw_game_mode (Variables|Default|GetPoints)))))))))))))

(event EventBeginPlay
  (bind _sphere (Variables|Default|GetSphere))
  (bind _returnvalue (Transformation|GetWorldLocation _sphere))
  ;[1 1 1] setting the world location
  (Transformation|SetWorldLocation _sphere (Math|Vector|MakeVector (.x _returnvalue) (.y _returnvalue) (.z _returnvalue)) false false))

(event EventTick
  (params (DeltaSeconds :type Float%20%28single-precision%29)))

(fn ConstructionScript)