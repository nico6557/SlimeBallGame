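; SlimeProjectile is a slime projectile actor that is mostly unfinished, with little active behavior.
; On BeginPlay it re-applies the Projectile component's current world location and halves the actor's scale.
; The component's overlap event is empty.
; Disconnected nodes hold unused logic for spawning another projectile, applying a zero impulse, and reacting to block hits with a material swap or a delayed destroy and break sound.
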(event OnComponentBeginOverlap(projectile)
  (params (OverlappedComponent :type Primitive%20Component%20Object%20Reference) (OtherActor :type Actor%20Object%20Reference) (OtherComp :type Primitive%20Component%20Object%20Reference) (OtherBodyIndex :type Integer) (bFromSweep :type Boolean) (SweepResult :type Hit%20Result%20Structure%20%28by%20ref%29))
  ;[1 1 1] DOESNT DO ANYTHING RN
)

(event EventBeginPlay
  (bind _projectile (Variables|Default|Getprojectile))
  (bind _returnvalue (Transformation|GetWorldLocation _projectile))
  ;[1 1 1] settign worl location of the slime
  (Transformation|SetWorldLocation _projectile (Math|Vector|MakeVector (.x _returnvalue) (.y _returnvalue) (.z _returnvalue)) false false)
  (Transformation|SetActorScale3D "0.500000,0.500000,0.500000"))

(event Collision|EventActorBeginOverlap
  (params (OtherActor :type Actor%20Object%20Reference)))

(event EventTick
  (params (DeltaSeconds :type Float%20%28single-precision%29)))

(fn ConstructionScript)