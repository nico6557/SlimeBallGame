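; Player controller that fires slimes from the mainPlayer pawn and keeps the mouse cursor visible.
; A looping MultiGate on Shoot cycles hero, fire, radioactive and lightning slimes, launched by impulse along the pawn's Angle component, copying each material onto the pawn.
; Follow-up presses spawn a second hero slime, scatter small fire slimes or dash the lightning slime; radioactive has none.
; MoveAim is empty, and older projectile and aiming drafts are disconnected.
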(event EventTick
  (params (DeltaSeconds :type Float%20%28single-precision%29))
  (Variables|Default|SetbShowMouseCursor true))

(event Input|ActionEvents|InputActionShoot
  (params (Key :type Key%20Structure :default "None"))
  ;[1 1 1] spawning hero slime
  (:Pressed
    (Utilities|FlowControl|MultiGate false true 0
      (:Out%200
        (bind _asmain_player (Utilities|Casting|CastTomainPlayer (Pawn|GetControlledPawn)))
        (bind _returnvalue (Game|SpawnActorfromClass "/Game/Blueprints/heroSlimeBP.heroSlimeBP_C" (Math|Transform|MakeTransform (.location (Transformation|GetWorldTransform (Variables|/Game/Blueprints/mainPlayer.mainPlayer_C|Getangle _asmain_player))) "0, 0, 0" "1,1,1") "Undefined" 0 0))
        (Physics|AddImpulse (Variables|/Game/Blueprints/heroSlimeBP.heroSlimeBP_C|GetSphere _returnvalue) (Math|Vector|RotateVector (Math|Vector|MakeVector 1e+05 0.0 0.0) (Transformation|GetWorldRotation (Variables|/Game/Blueprints/mainPlayer.mainPlayer_C|Getangle _asmain_player))) "None" false)
        (Rendering|Material|SetMaterial (Variables|/Game/Blueprints/mainPlayer.mainPlayer_C|GetSphere (stale _asmain_player_2)) 0 (Rendering|Material|GetMaterial (Variables|/Game/Blueprints/heroSlimeBP.heroSlimeBP_C|GetSphere _returnvalue) 0))
        (bind _asmain_player_2 (Utilities|Casting|CastTomainPlayer (Pawn|GetControlledPawn))))
      (:Out%201
        ;[1 1 1] spawning a second one when spacebar is hit a second time
        (bind _returnvalue_2 (Game|SpawnActorfromClass "/Game/Blueprints/heroSlimeBP.heroSlimeBP_C" (Math|Transform|MakeTransform (Transformation|GetWorldLocation (Variables|/Game/Blueprints/heroSlimeBP.heroSlimeBP_C|GetSphere _returnvalue)) "0, 0, 0" "1,1,1") "Undefined" 0 0))
        (Physics|AddImpulse (Variables|/Game/Blueprints/heroSlimeBP.heroSlimeBP_C|GetSphere _returnvalue_2) (Math|Vector|MakeVector 3e+03 0.0 0.0) "None" false))
      (:Out%202
        ;[1 1 1] spawning fire slime
        (bind _asmain_player_3 (Utilities|Casting|CastTomainPlayer (Pawn|GetControlledPawn)))
        (bind _returnvalue_3 (Game|SpawnActorfromClass "/Game/Blueprints/fireSlimeBP.fireSlimeBP_C" (Math|Transform|MakeTransform (.location (Transformation|GetWorldTransform (Variables|/Game/Blueprints/mainPlayer.mainPlayer_C|Getangle _asmain_player_3))) "0, 0, 0" "1,1,1") "Undefined" 0 0))
        (Physics|AddImpulse (Variables|/Game/Blueprints/fireSlimeBP.fireSlimeBP_C|GetSphere _returnvalue_3) (Math|Vector|RotateVector (Math|Vector|MakeVector 1e+05 0.0 0.0) (Transformation|GetWorldRotation (Variables|/Game/Blueprints/mainPlayer.mainPlayer_C|Getangle _asmain_player_3))) "None" false)
        (Rendering|Material|SetMaterial (Variables|/Game/Blueprints/mainPlayer.mainPlayer_C|GetSphere (stale _asmain_player_4)) 0 (Rendering|Material|GetMaterial (Variables|/Game/Blueprints/fireSlimeBP.fireSlimeBP_C|GetSphere _returnvalue_3) 0))
        (bind _asmain_player_4 (Utilities|Casting|CastTomainPlayer (Pawn|GetControlledPawn))))
      (:Out%203
        ;[1 1 1] spawning a second one when spacebar is hit a second time
        (for _index (range 0 7)
          (bind _returnvalue_4 (Game|SpawnActorfromClass "/Game/Blueprints/smallFireSlimeBP.smallFireSlimeBP_C" (Math|Transform|MakeTransform (+ (Transformation|GetWorldLocation (Variables|/Game/Blueprints/fireSlimeBP.fireSlimeBP_C|GetSphere _returnvalue_3)) (Math|Float|Truncate (Math|Random|RandomFloatinRange -1e+01 1e+01))) "0, 0, 0" "0.100000,0.100000,0.100000") "Undefined" 0 0))
          (Physics|AddImpulse (Variables|/Game/Blueprints/smallFireSlimeBP.smallFireSlimeBP_C|GetSphere _returnvalue_4) (Math|Vector|MakeVector (Math|Conversions|ToFloat(Integer) (Math|Random|RandomInteger 2000)) 0.0 0.0) "None" false)))
      (:Out%204
        ;[1 1 1] spawning raidioctive slime
        (bind _asmain_player_5 (Utilities|Casting|CastTomainPlayer (Pawn|GetControlledPawn)))
        (bind _returnvalue_5 (Game|SpawnActorfromClass "/Game/Blueprints/radioactiveSlimeBP.radioactiveSlimeBP_C" (Math|Transform|MakeTransform (.location (Transformation|GetWorldTransform (Variables|/Game/Blueprints/mainPlayer.mainPlayer_C|Getangle _asmain_player_5))) "0, 0, 0" "1,1,1") "Undefined" 0 0))
        (Physics|AddImpulse (Variables|/Game/Blueprints/radioactiveSlimeBP.radioactiveSlimeBP_C|GetSphere _returnvalue_5) (Math|Vector|RotateVector (Math|Vector|MakeVector 1e+05 0.0 0.0) (Transformation|GetWorldRotation (Variables|/Game/Blueprints/mainPlayer.mainPlayer_C|Getangle _asmain_player_5))) "None" false)
        (Rendering|Material|SetMaterial (Variables|/Game/Blueprints/mainPlayer.mainPlayer_C|GetSphere (stale _asmain_player_6)) 0 (Rendering|Material|GetMaterial (Variables|/Game/Blueprints/radioactiveSlimeBP.radioactiveSlimeBP_C|GetSphere _returnvalue_5) 0))
        (bind _asmain_player_6 (Utilities|Casting|CastTomainPlayer (Pawn|GetControlledPawn))))
      (:Out%205
        ;[1 1 1] spawning lightning slime
        (bind _asmain_player_7 (Utilities|Casting|CastTomainPlayer (Pawn|GetControlledPawn)))
        (bind _returnvalue_6 (Game|SpawnActorfromClass "/Game/Blueprints/lightningSlimeBP.lightningSlimeBP_C" (Math|Transform|MakeTransform (.location (Transformation|GetWorldTransform (Variables|/Game/Blueprints/mainPlayer.mainPlayer_C|Getangle _asmain_player_7))) "0, 0, 0" "1,1,1") "Undefined" 0 0))
        (Physics|AddImpulse (Variables|/Game/Blueprints/lightningSlimeBP.lightningSlimeBP_C|GetSphere _returnvalue_6) (Math|Vector|RotateVector (Math|Vector|MakeVector 1e+05 0.0 0.0) (Transformation|GetWorldRotation (Variables|/Game/Blueprints/mainPlayer.mainPlayer_C|Getangle _asmain_player_7))) "None" false)
        (Rendering|Material|SetMaterial (Variables|/Game/Blueprints/mainPlayer.mainPlayer_C|GetSphere (stale _asmain_player_8)) 0 (Rendering|Material|GetMaterial (Variables|/Game/Blueprints/lightningSlimeBP.lightningSlimeBP_C|GetSphere _returnvalue_6) 0))
        (bind _asmain_player_8 (Utilities|Casting|CastTomainPlayer (Pawn|GetControlledPawn))))
      (:Out%206
        ;[1 1 1] makes it go quick in the direction you are pointing
        (Physics|AddImpulse (Variables|/Game/Blueprints/lightningSlimeBP.lightningSlimeBP_C|GetSphere _returnvalue_6) (Math|Vector|RotateVector (Math|Vector|MakeVector 1e+06 0.0 0.0) (Transformation|GetWorldRotation (Variables|/Game/Blueprints/mainPlayer.mainPlayer_C|Getangle _asmain_player_7))) "None" false)))))

(event Input|ActionEvents|InputActionShoot
  (params (Key :type Key%20Structure :default "None"))
  ;[1 1 1] first draft
)

(event Input|AxisEvents|InputAxisMoveAim
  (params (AxisValue :type Float%20%28single-precision%29))
  ;[1 1 1] first draft of moving with keys
)

(fn ConstructionScript)