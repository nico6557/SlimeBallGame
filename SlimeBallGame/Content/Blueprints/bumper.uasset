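; A bumper actor that knocks slime projectiles away when they overlap its Sphere component.
; On overlap it plays a block-break sound and applies a BumpPower-scaled impulse to the projectile.
; The impulse points away from a spot 50 units above the bumper's origin toward the projectile.
; BeginPlay re-sets the Sphere to its own current world location, so it has no apparent effect.
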(event OnComponentBeginOverlap(Sphere)
  (params (OverlappedComponent :type Primitive%20Component%20Object%20Reference) (OtherActor :type Actor%20Object%20Reference) (OtherComp :type Primitive%20Component%20Object%20Reference) (OtherBodyIndex :type Integer) (bFromSweep :type Boolean) (SweepResult :type Hit%20Result%20Structure%20%28by%20ref%29))
  (bind _returnvalue (Transformation|GetActorLocation))
  ;[1 1 1] bump
  (bind _asslime_projectile (Utilities|Casting|CastToSlimeProjectile OtherActor))
  (Audio|PlaySoundatLocation "/Game/Sounds/blockBreakCue.blockBreakCue" _returnvalue "0, 0, 0" 1.0 1.0 0.0 0 0 0)
  (Physics|AddImpulse (Variables|/Game/Blueprints/SlimeProjectile.SlimeProjectile_C|Getprojectile _asslime_projectile) (* (Math|Vector|Normalize (- (Transformation|GetActorLocation _asslime_projectile) (+ _returnvalue "0, 0,50.000000"))) (Variables|Default|GetbumpPower)) "None" false))

(event EventBeginPlay
  (bind _sphere (Variables|Default|GetSphere))
  (bind _returnvalue (Transformation|GetWorldLocation _sphere))
  ;[1 1 1] setting the world location
  (Transformation|SetWorldLocation _sphere (Math|Vector|MakeVector (.x _returnvalue) (.y _returnvalue) (.z _returnvalue)) false false))

(event EventTick
  (params (DeltaSeconds :type Float%20%28single-precision%29)))

(fn ConstructionScript)