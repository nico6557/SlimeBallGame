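; Player controller for a slime-launching game that shows the cursor and fires slimes from the mainPlayer's Angle component on Shoot.
; A looping MultiGate sequences presses through hero, fire, radioactive and lightning slimes, swapping the pawn's material after each launch.
; Follow-up presses trigger live-slime abilities: hero duplicates, fire bursts into small slimes, lightning dashes along the aim; radioactive has none.
; If the hero or fire slime is gone, that press launches the next type instead.
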(event EventBeginPlay
  (bind _assaw_game_mode (Utilities|Casting|CastTosawGameMode (Game|GetGameMode)))
  (Variables|Default|SetAs%20Saw%20Game%20Mode _assaw_game_mode)
  (bind _asmain_player (Utilities|Casting|CastTomainPlayer (Pawn|GetControlledPawn)))
  (Rendering|Material|SetMaterial (Variables|/Game/Blueprints/mainPlayer.mainPlayer_C|GetSphere _asmain_player) 0 "/Game/Materials/heroSlimeMAT.heroSlimeMAT"))

(event EventTick
  (params (DeltaSeconds :type Float%20%28single-precision%29))
  (Variables|Default|SetbShowMouseCursor true))

(event Input|ActionEvents|InputActionShoot
  (params (Key :type Key%20Structure :default "None"))
  ;[1 1 1] spawning hero slime
  (:Pressed
    (Utilities|FlowControl|MultiGate false true (Variables|Default|GetIndex) :!label _label
      (:Out%200
        (bind _asmain_player (Utilities|Casting|CastTomainPlayer (Pawn|GetControlledPawn)))
        (bind _returnvalue (Game|SpawnActorfromClass "/Game/Blueprints/heroSlimeBP.heroSlimeBP_C" (Math|Transform|MakeTransform (.location (Transformation|GetWorldTransform (Variables|/Game/Blueprints/mainPlayer.mainPlayer_C|Getangle _asmain_player))) "0, 0, 0" "1,1,1") "Undefined" 0 0))
        (Physics|AddImpulse (Variables|/Game/Blueprints/heroSlimeBP.heroSlimeBP_C|GetSphere _returnvalue) (Math|Vector|RotateVector (Math|Vector|MakeVector 1e+05 0.0 0.0) (Transformation|GetWorldRotation (Variables|/Game/Blueprints/mainPlayer.mainPlayer_C|Getangle _asmain_player))) "None" false)
        (bind _asmain_player_2 (Utilities|Casting|CastTomainPlayer (Pawn|GetControlledPawn)))
        (Rendering|Material|SetMaterial (Variables|/Game/Blueprints/mainPlayer.mainPlayer_C|GetSphere _asmain_player_2) 0 "/Game/Materials/fireSlimeMAT.fireSlimeMAT"))
      (:Out%201
        (Utilities|IsValid (Variables|/Game/Blueprints/heroSlimeBP.heroSlimeBP_C|GetSphere _returnvalue)
          (:Is%20Valid
            ;[1 1 1] spawning a second one when spacebar is hit a second time
            (bind _returnvalue_2 (Game|SpawnActorfromClass "/Game/Blueprints/heroSlimeBP.heroSlimeBP_C" (Math|Transform|MakeTransform (Transformation|GetWorldLocation (Variables|/Game/Blueprints/heroSlimeBP.heroSlimeBP_C|GetSphere _returnvalue)) "0, 0, 0" "1,1,1") "Undefined" 0 0))
            (Physics|AddImpulse (Variables|/Game/Blueprints/heroSlimeBP.heroSlimeBP_C|GetSphere _returnvalue_2) (Math|Vector|MakeVector 3e+03 0.0 0.0) "None" false)
            (Audio|PlaySoundatLocation "/Game/Sounds/heroBloop_Cue.heroBloop_Cue" "0, 0, 0" "0, 0, 0" 1.0 1.0 0.0 0 0 0))
          (:Is%20Not%20Valid
            (Variables|Default|SetIndex 4)
            ;[1 1 1] spawning fire slime
            (bind _asmain_player_3 (Utilities|Casting|CastTomainPlayer (Pawn|GetControlledPawn) :!label _label_2))
            (bind _returnvalue_3 (Game|SpawnActorfromClass "/Game/Blueprints/fireSlimeBP.fireSlimeBP_C" (Math|Transform|MakeTransform (.location (Transformation|GetWorldTransform (Variables|/Game/Blueprints/mainPlayer.mainPlayer_C|Getangle _asmain_player_3))) "0, 0, 0" "1,1,1") "Undefined" 0 0))
            (Physics|AddImpulse (Variables|/Game/Blueprints/fireSlimeBP.fireSlimeBP_C|GetSphere _returnvalue_3) (Math|Vector|RotateVector (Math|Vector|MakeVector 1e+05 0.0 0.0) (Transformation|GetWorldRotation (Variables|/Game/Blueprints/mainPlayer.mainPlayer_C|Getangle _asmain_player_3))) "None" false)
            (bind _asmain_player_4 (Utilities|Casting|CastTomainPlayer (Pawn|GetControlledPawn)))
            (Rendering|Material|SetMaterial (Variables|/Game/Blueprints/mainPlayer.mainPlayer_C|GetSphere _asmain_player_4) 0 "/Game/Materials/greenSlimeMAT.greenSlimeMAT"))))
      (:Out%202
        (goto _label_2))
      (:Out%203
        (Utilities|IsValid (Variables|/Game/Blueprints/fireSlimeBP.fireSlimeBP_C|GetSphere _returnvalue_3)
          (:Is%20Valid
            ;[1 1 1] spawning a second one when spacebar is hit a second time
            (for _index (range 0 7)
              (bind _returnvalue_4 (Game|SpawnActorfromClass "/Game/Blueprints/smallFireSlimeBP.smallFireSlimeBP_C" (Math|Transform|MakeTransform (+ (Transformation|GetWorldLocation (Variables|/Game/Blueprints/fireSlimeBP.fireSlimeBP_C|GetSphere _returnvalue_3)) (Math|Float|Truncate (Math|Random|RandomFloatinRange -1e+01 1e+01))) "0, 0, 0" "0.100000,0.100000,0.100000") "AdjustIfPossibleButAlwaysSpawn" 0 0))
              (Physics|AddImpulse (Variables|/Game/Blueprints/smallFireSlimeBP.smallFireSlimeBP_C|GetSphere _returnvalue_4) (Math|Vector|MakeVector (Math|Conversions|ToFloat(Integer) (Math|Random|RandomInteger 2000)) 0.0 0.0) "None" false)
              (Audio|PlaySoundatLocation "/Game/StarterContent/Audio/Explosion01.Explosion01" "0, 0, 0" "0, 0, 0" 1.0 1.0 0.0 0 0 0)))
          (:Is%20Not%20Valid
            (Variables|Default|SetIndex 5)
            ;[1 1 1] spawning raidioctive slime
            (bind _asmain_player_5 (Utilities|Casting|CastTomainPlayer (Pawn|GetControlledPawn) :!label _label_3))
            (bind _returnvalue_5 (Game|SpawnActorfromClass "/Game/Blueprints/radioactiveSlimeBP.radioactiveSlimeBP_C" (Math|Transform|MakeTransform (.location (Transformation|GetWorldTransform (Variables|/Game/Blueprints/mainPlayer.mainPlayer_C|Getangle _asmain_player_5))) "0, 0, 0" "1,1,1") "Undefined" 0 0))
            (Physics|AddImpulse (Variables|/Game/Blueprints/radioactiveSlimeBP.radioactiveSlimeBP_C|GetSphere _returnvalue_5) (Math|Vector|RotateVector (Math|Vector|MakeVector 1e+05 0.0 0.0) (Transformation|GetWorldRotation (Variables|/Game/Blueprints/mainPlayer.mainPlayer_C|Getangle _asmain_player_5))) "None" false)
            (bind _asmain_player_6 (Utilities|Casting|CastTomainPlayer (Pawn|GetControlledPawn)))
            (Rendering|Material|SetMaterial (Variables|/Game/Blueprints/mainPlayer.mainPlayer_C|GetSphere _asmain_player_6) 0 "/Game/Materials/lighningSlimeMAT.lighningSlimeMAT"))))
      (:Out%204
        (goto _label_3))
      (:Out%205
        ;[1 1 1] spawning lightning slime
        (bind _asmain_player_7 (Utilities|Casting|CastTomainPlayer (Pawn|GetControlledPawn)))
        (bind _returnvalue_6 (Game|SpawnActorfromClass "/Game/Blueprints/lightningSlimeBP.lightningSlimeBP_C" (Math|Transform|MakeTransform (.location (Transformation|GetWorldTransform (Variables|/Game/Blueprints/mainPlayer.mainPlayer_C|Getangle _asmain_player_7))) "0, 0, 0" "1,1,1") "Undefined" 0 0))
        (Physics|AddImpulse (Variables|/Game/Blueprints/lightningSlimeBP.lightningSlimeBP_C|GetSphere _returnvalue_6) (Math|Vector|RotateVector (Math|Vector|MakeVector 1e+05 0.0 0.0) (Transformation|GetWorldRotation (Variables|/Game/Blueprints/mainPlayer.mainPlayer_C|Getangle _asmain_player_7))) "None" false)
        (bind _asmain_player_8 (Utilities|Casting|CastTomainPlayer (Pawn|GetControlledPawn)))
        (Rendering|Material|SetMaterial (Variables|/Game/Blueprints/mainPlayer.mainPlayer_C|GetSphere _asmain_player_8) 0 "/Game/Materials/heroSlimeMAT.heroSlimeMAT"))
      (:Out%206
        (Utilities|IsValid (Variables|/Game/Blueprints/lightningSlimeBP.lightningSlimeBP_C|GetSphere _returnvalue_6)
          (:Is%20Valid
            ;[1 1 1] makes it go quick in the direction you are pointing
            (Physics|AddImpulse (Variables|/Game/Blueprints/lightningSlimeBP.lightningSlimeBP_C|GetSphere _returnvalue_6) (Math|Vector|RotateVector (Math|Vector|MakeVector 1e+06 0.0 0.0) (Transformation|GetWorldRotation (Variables|/Game/Blueprints/mainPlayer.mainPlayer_C|Getangle _asmain_player_7))) "None" false)
            (Audio|PlaySoundatLocation "/Game/Sounds/zapCue.zapCue" "0, 0, 0" "0, 0, 0" 1.0 1.0 0.0 0 0 0)
            (Variables|Default|SetIndex 0)
            (goto _label Reset))
          (:Is%20Not%20Valid
            (Variables|Default|SetIndex 0)
            (goto _label Reset)))))))

(fn ConstructionScript)