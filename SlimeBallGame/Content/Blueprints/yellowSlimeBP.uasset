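; Yellow slime actor built around a Sphere component, apparently an unfinished projectile for mainPlayer to shoot.
; BeginPlay sets the sphere's world location to its current position, so it stays in place.
; The Shoot input casts the Instigator's controlled pawn to mainPlayer but does nothing further.
; A disconnected AddImpulse would launch the sphere along a fixed vector rotated by the player's Angle component, but it never runs.
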(event Collision|EventActorBeginOverlap
  (params (OtherActor :type Actor%20Object%20Reference)))

(event EventTick
  (params (DeltaSeconds :type Float%20%28single-precision%29)))

(event EventBeginPlay
  (bind _sphere (Variables|Default|GetSphere))
  (bind _returnvalue (Transformation|GetWorldLocation _sphere))
  (Transformation|SetWorldLocation _sphere (Math|Vector|MakeVector (.x _returnvalue) (.y _returnvalue) (.z _returnvalue)) false false))

(event Input|ActionEvents|InputActionShoot
  (params (Key :type Key%20Structure))
  (:Pressed
    (bind _asmain_player (Utilities|Casting|CastTomainPlayer (Pawn|GetControlledPawn (Pawn|GetController (Variables|Actor|GetInstigator)))))))

(fn ConstructionScript)