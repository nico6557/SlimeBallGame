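; Breakable block actor that reacts to SlimeProjectile overlaps on its Rr component.
; While SecondHit is true, a hit swaps the Break component's material to M_AssetPlatform and clears the flag.
; A hit with the flag cleared waits briefly, destroys the actor, then plays BloopCue at Break's location.
; BeginPlay re-applies Rr's current world location, leaving its position unchanged.
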(event OnComponentBeginOverlap(rr)
  (params (OverlappedComponent :type Primitive%20Component%20Object%20Reference) (OtherActor :type Actor%20Object%20Reference) (OtherComp :type Primitive%20Component%20Object%20Reference) (OtherBodyIndex :type Integer) (bFromSweep :type Boolean) (SweepResult :type Hit%20Result%20Structure%20%28by%20ref%29))
  ;[1 1 1] on second hit the sphere breaks playiong a noise
  (Utilities|Casting|CastToSlimeProjectile OtherActor)
  (if (Variables|Default|GetsecondHit)
    (Rendering|Material|SetMaterial (Variables|Default|Getbreak) 0 "/Game/StarterContent/Materials/M_AssetPlatform.M_AssetPlatform")
    (Variables|Default|SetsecondHit false)
    (else
      (Utilities|FlowControl|Delay 0.1)
      (Actor|DestroyActor self)
      (Audio|PlaySoundatLocation "/Game/Sounds/bloopCue.bloopCue" (Transformation|GetWorldLocation (Variables|Default|Getbreak)) "0, 0, 0" 1.0 1.0 0.0 0 0 0))))

(event EventBeginPlay
  (bind _rr (Variables|Default|Getrr))
  (bind _returnvalue (Transformation|GetWorldLocation _rr))
  ;[1 1 1] setting the world location
  (Transformation|SetWorldLocation _rr (Math|Vector|MakeVector (.x _returnvalue) (.y _returnvalue) (.z _returnvalue)) false false))

(event EventTick
  (params (DeltaSeconds :type Float%20%28single-precision%29)))

(fn ConstructionScript)